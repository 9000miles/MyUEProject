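; Game settings manager that stores, saves and applies player language and gamma settings.
; The set function writes settings into the current save data, optionally pushing them to GameInit and saving to slot.
; On BeginPlay it binds two refresh events to GameInit's setting-change event.
; These notify language-interface widgets and write gamma to a tagged PostProcessVolume.
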(event `Event_RefreshLanguageText`
  (`self.Mac_RefreshLanguageText`))

(event `self.ReceiveBeginPlay`
  (bind _angameinit (`/Game/BluePrints/FunctionLibraryBP/GameSaveData_FL.Method_GetGameInit`))
  (`|ExecutionSequence`
    (:`then_0`
      (add `CreateSaveGamedataManager.OnSettingDataChangeEvent` _angameinit (delegate `Event_RefreshLanguageText`)))
    (:`then_1`
      (add `CreateSaveGamedataManager.OnSettingDataChangeEvent` _angameinit (delegate `Event_RefreshGammeValue`)))))

(event `Event_RefreshGammeValue`
  (`self.Mac_RefreshGammeValue`))

(fn `Func_GetGameSettings`
  (returns (gsv_GameSettings :type "/Game/DataConfig/Struct/Struct_GameSettings Structure"))
  (bind _curgamesavedata (`/Game/BluePrints/FunctionLibraryBP/GameSaveData_FL.Method_GetCurGameSaveData`))
  (return (`/Game/DataConfig/GlobalData/SettingSaveData_BP.gsv_GameSettings` _curgamesavedata)))

(fn `Func_SetGameSettings`
  (params (InSettings :type "/Game/DataConfig/Struct/Struct_GameSettings Structure") (IsNeedSave :type Boolean :default true))
  (bind _output_get (set `self.var_CurGameSettings` InSettings))
  (bind _gsv_gamesettings (`self.Func_GetGameSettings`))
  (set `self.var_OldGameSettings` _gsv_gamesettings)
  (bind _curgamesavedata (`/Game/BluePrints/FunctionLibraryBP/GameSaveData_FL.Method_GetCurGameSaveData`))
  (set `/Game/DataConfig/GlobalData/SettingSaveData_BP.gsv_GameSettings` _output_get _curgamesavedata)
  (set `SettingSaveData.LanguageEnum` (`.gsv_Language_22_98F99208485746BEAA7EB7A11C8C7C89` (break `/Game/DataConfig/Struct/Struct_GameSettings` (`self.var_CurGameSettings`))) _curgamesavedata)
  (if (`local.IsNeedSave`)
    (bind _angameinit (`/Game/BluePrints/FunctionLibraryBP/GameSaveData_FL.Method_GetGameInit`))
    (bind _curgamesavedata_2 (`/Game/BluePrints/FunctionLibraryBP/GameSaveData_FL.Method_GetCurGameSaveData`))
    (`CreateSaveGamedataManager.SetGameSettingData` _angameinit _curgamesavedata_2)
    (`GameplayStatics.SaveGameToSlot` _curgamesavedata_2 (`SettingSaveData.SaveSlotName` _curgamesavedata_2) (`KismetMathLibrary.Conv_ByteToInt` (`SettingSaveData.UserIndex` _curgamesavedata_2)))
    (set `/Game/BluePrints/MainBP/GameInit.var_CurGameData` _curgamesavedata_2 _angameinit)))

(fn `UserConstructionScript`)