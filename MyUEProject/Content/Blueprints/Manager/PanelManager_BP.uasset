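; PanelManager_BP is a manager Blueprint that handles UI panel navigation through a PanelHistory stack.
; OpenPage opens and pushes a panel, then closes the one beneath it.
; ClosePage closes and removes the top panel, then reopens the previous one.
; Its event handlers are empty, and the test logic that creates random numbered panels with open/close callbacks is disconnected, as are the debug prints.
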(event `CustomEvent_1`)

(event `Key|Add`
  (params (Key :type "Key Structure")))

(event `CustomEvent_3`)

(event `Key|Subtract`
  (params (Key :type "Key Structure")))

(event `self.ReceiveTick`
  (params (DeltaSeconds :type "Float (single-precision)")))

(event `self.ReceiveBeginPlay`)

(event `Key|NumPadEight`
  (params (Key :type "Key Structure")))

(fn `ClosePage`
  (locals (LV_Index :type Integer))
  (bind _panelhistory (`self.PanelHistory`))
  (bind _lv_index (`local.LV_Index`))
  (bind _result (`/Engine/EditorBlueprintResources/StandardMacros.DecrementInt` (`KismetArrayLibrary.Array_Length` (`self.PanelHistory`)))
    (:`  `
      (bind _output_get (set `local.LV_Index` _result))
      (if (>= _result 0)
        (set `self.CurIndex` _output_get)
        (`/Game/UIWidget/Panel/PanelBase.Close` (`|GetArrayItem` _panelhistory _lv_index))
        (if (>= (`KismetArrayLibrary.Array_Length` _panelhistory) 2)
          (`/Game/UIWidget/Panel/PanelBase.Open` (`|GetArrayItem` _panelhistory (- _lv_index 1))))
        (`KismetArrayLibrary.Array_Remove` (`self.PanelHistory`) (`local.LV_Index`))))))

(fn `OpenPage`
  (params (Page :type "/Game/UIWidget/Panel/PanelBase Object Reference (by ref)"))
  (locals (LV_Index :type Integer :default 0))
  (bind _panelhistory (`self.PanelHistory`))
  (bind _panelhistory_2 (`self.PanelHistory`))
  (`/Game/UIWidget/Panel/PanelBase.Open` Page)
  (bind _returnvalue (`KismetArrayLibrary.Array_Add` _panelhistory Page))
  (bind _output_get (set `local.LV_Index` _returnvalue))
  (set `self.CurIndex` _output_get)
  (if (>= (`KismetArrayLibrary.Array_Length` _panelhistory) 2)
    (`/Game/UIWidget/Panel/PanelBase.Close` (`|GetArrayItem` _panelhistory_2 (- (`KismetArrayLibrary.Array_Length` _panelhistory_2) 2)))))

(fn `UserConstructionScript`)