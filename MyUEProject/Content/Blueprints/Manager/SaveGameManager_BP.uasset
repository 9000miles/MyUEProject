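; Save manager Blueprint that keeps named, typed values in a map of SaveDataObject_BP objects, with functions to add, get, set and remove them.
; Saving flattens the map into one delimited string inside a SaveGame_BP, stored by slot name and user index; loading parses it to rebuild the map.
; Hard-coded debug keys save and delete test slots, while numpad keys exercise a separate SaveGameManager() API.
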(event `Key|NumPadTwo`
  (params (Key :type "Key Structure"))
  (:`Pressed`
    (`SaveGameManager.SetSaveDataValue` (subsystem `SaveGameManager`) "SaveData_01" "Int32" "656" "Default" false)))

(event `Key|NumPadZero`
  (params (Key :type "Key Structure"))
  (:`Pressed`
    (bind _output_get (set `self.CurSlotName` "MyUEProject"))
    (bind _output_get_2 (set `self.CurUserIndex` 0))
    (`SaveGameManager.SaveGameData` (subsystem `SaveGameManager`) _output_get _output_get_2)))

(event `Key|NumPadOne`
  (params (Key :type "Key Structure"))
  (:`Pressed`
    (`SaveGameManager.LoadGameData` (subsystem `SaveGameManager`) "MyUEProject" 0)))

(event `self.ReceiveBeginPlay`)

(event `self.ReceiveDestroyed`)

(event `Key|Zero`
  (params (Key :type "Key Structure"))
  (:`Pressed`
    (bind _output_get (set `self.CurSlotName` "MySaveGame"))
    (bind _output_get_2 (set `self.CurUserIndex` 0))
    (`self.SaveGameData` _output_get _output_get_2)))

(event `Key|One`
  (params (Key :type "Key Structure"))
  (:`Pressed`
    (bind _output_get (set `self.CurSlotName` "MySaveGame"))
    (bind _output_get_2 (set `self.CurUserIndex` 1))
    (`self.SaveGameData` _output_get _output_get_2)))

(event `Key|Two`
  (params (Key :type "Key Structure"))
  (:`Pressed`
    (bind _output_get (set `self.CurSlotName` "MySaveGame"))
    (bind _output_get_2 (set `self.CurUserIndex` 2))
    (`self.SaveGameData` _output_get _output_get_2)))

(event `Key|Five`
  (params (Key :type "Key Structure"))
  (:`Pressed`
    (bind _output_get (set `self.CurSlotName` "LiZiJun"))
    (bind _output_get_2 (set `self.CurUserIndex` 0))
    (`self.SaveGameData` _output_get _output_get_2)))

(event `Key|Six`
  (params (Key :type "Key Structure"))
  (:`Pressed`
    (bind _output_get (set `self.CurSlotName` "LiZiJun"))
    (bind _output_get_2 (set `self.CurUserIndex` 1))
    (`self.SaveGameData` _output_get _output_get_2)))

(event `Key|SpaceBar`
  (params (Key :type "Key Structure")))

(event `CustomEvent_0`
  (params (Value :type String)))

(event `Key|F`
  (params (Key :type "Key Structure"))
  (:`Pressed`
    (`self.DeleteGameData` "LiZiJun")))

(event `Key|H`
  (params (Key :type "Key Structure"))
  (:`Pressed`
    (`self.DeleteGameData` "MySaveGame" 1)))

(fn `AddData`
  (params (DataName :type String) (DataType :type "/Game/Blueprints/SaveGame/ESaveGameData Enum" :default "NewEnumerator0") (String :type String) (Integer :type Integer) (Float :type "Float (double-precision)") (Boolean :type Boolean) (Vector :type "Vector Structure"))
  (locals (LV_Data :type "/Game/Blueprints/SaveGame/SaveDataObject_BP Object Reference"))
  (bind _dataname (`local.DataName`))
  (bind _dataname_2 (`local.DataName`))
  (bind _dataname_3 (`local.DataName`))
  (bind _dataname_4 (`local.DataName`))
  (bind _dataname_5 (`local.DataName`))
  (if (not (`.ReturnValue` (`BlueprintMapLibrary.Map_Find` (`self.SaveDatas`) DataName)))
    (switch `/Game/Blueprints/SaveGame/ESaveGameData` (`local.DataType`)
      (:`NewEnumerator0`
        (bind _returnvalue (`|GenericCreateObject` "/Game/Blueprints/SaveGame/SaveDataObject_BP.SaveDataObject_BP_C" self _dataname_3 "NewEnumerator0" (`local.String`)))
        (`BlueprintMapLibrary.Map_Add` (`self.SaveDatas`) _dataname_3 _returnvalue))
      (:`NewEnumerator1`
        (bind _returnvalue_2 (`|GenericCreateObject` "/Game/Blueprints/SaveGame/SaveDataObject_BP.SaveDataObject_BP_C" self _dataname_4 "NewEnumerator1" "" (`local.Integer`)))
        (`BlueprintMapLibrary.Map_Add` (`self.SaveDatas`) _dataname_4 _returnvalue_2))
      (:`NewEnumerator2`
        (bind _returnvalue_3 (`|GenericCreateObject` "/Game/Blueprints/SaveGame/SaveDataObject_BP.SaveDataObject_BP_C" self _dataname_5 "NewEnumerator2" "" 0 (`local.Float`)))
        (`BlueprintMapLibrary.Map_Add` (`self.SaveDatas`) _dataname_5 _returnvalue_3))
      (:`NewEnumerator3`
        (bind _returnvalue_4 (`|GenericCreateObject` "/Game/Blueprints/SaveGame/SaveDataObject_BP.SaveDataObject_BP_C" self _dataname "NewEnumerator3" "" 0 0.0 (`local.Boolean`)))
        (`BlueprintMapLibrary.Map_Add` (`self.SaveDatas`) _dataname _returnvalue_4))
      (:`NewEnumerator4`
        (bind _returnvalue_5 (`|GenericCreateObject` "/Game/Blueprints/SaveGame/SaveDataObject_BP.SaveDataObject_BP_C" self _dataname_2 "NewEnumerator4" "" 0 0.0 false (`local.Vector`)))
        (`BlueprintMapLibrary.Map_Add` (`self.SaveDatas`) _dataname_2 _returnvalue_5)))
    (else
      (`KismetSystemLibrary.PrintString` (`KismetStringLibrary.Concat_StrStr` DataName " is alredy exist")))))

(fn `DeleteGameData`
  (params (SlotName :type String) (UserIndex :type Integer))
  (`GameplayStatics.DeleteGameInSlot` SlotName UserIndex))

(fn `GetData`
  (params (DataName :type String) (DataType :type "/Game/Blueprints/SaveGame/ESaveGameData Enum" :default "NewEnumerator0"))
  (returns (SaveDataObject :type "/Game/Blueprints/SaveGame/SaveDataObject_BP Object Reference"))
  (locals (LV_Data :type "/Game/Blueprints/SaveGame/SaveDataObject_BP Object Reference"))
  (bind _lv_data (`local.LV_Data`))
  (bind (_value _returnvalue) (`BlueprintMapLibrary.Map_Find` (`self.SaveDatas`) DataName))
  (if _returnvalue
    (`/Engine/EditorBlueprintResources/StandardMacros.IsValid` _value
      (:`Is Valid`
        (bind _output_get (set `local.LV_Data` _value))
        (if (`|EnumEquality` (`local.DataType`) (`/Game/Blueprints/SaveGame/SaveDataObject_BP.DataType` _output_get))
          (`/Game/Blueprints/SaveGame/SaveDataObject_BP.Event_ChangeValue` _lv_data _lv_data)
          (return (`local.LV_Data`))
          (else
            (`KismetSystemLibrary.PrintString` "SaveDataType not equal"))))
      (:`Is Not Valid`
        (`KismetSystemLibrary.PrintString` "SaveDataObject is not valid")))
    (else
      (`KismetSystemLibrary.PrintString` (`KismetStringLibrary.Concat_StrStr` DataName " not found")))))

(fn `LoadGameData`
  (params (SlotName :type String) (UserIndex :type Integer))
  (bind _returnvalue (`GameplayStatics.DoesSaveGameExist` SlotName UserIndex))
  (if _returnvalue
    (bind _returnvalue_2 (`GameplayStatics.LoadGameFromSlot` SlotName UserIndex))
    (bind _assave_game_bp (cast `/Game/Blueprints/SaveGame/SaveGame_BP` _returnvalue_2))
    (set `self.CurSaveGameObject` _assave_game_bp)
    (`self.StringToSaveDatas` (`/Game/Blueprints/SaveGame/SaveGame_BP.DataString` _assave_game_bp))
    (set `self.CurSlotName` (`local.SlotName`))
    (set `self.CurUserIndex` (`local.UserIndex`))
    (else
      (`KismetSystemLibrary.PrintString` (`KismetStringLibrary.Concat_StrStr` SlotName " " (`KismetStringLibrary.Conv_IntToString` UserIndex) " not exist"))
      (set `self.CurSlotName` (`local.SlotName`))
      (set `self.CurUserIndex` (`local.UserIndex`)))))

(fn `RemoveData`
  (params (DataName :type String))
  (`BlueprintMapLibrary.Map_Remove` (`self.SaveDatas`) DataName))

(fn `SaveDatasToString`
  (returns (ReturnValue :type String))
  (locals (LV_DataString :type String))
  (bind _values (`BlueprintMapLibrary.Map_Values` (`self.SaveDatas`)))
  (for _array_element _values
    (bind _output (`/Game/Blueprints/SaveGame/SaveDataObject_BP.DataToString` _array_element))
    (set `local.LV_DataString` (`KismetStringLibrary.Concat_StrStr` (`local.LV_DataString`) _output ";")))
  (return (`KismetStringLibrary.LeftChop` (`local.LV_DataString`) 1)))

(fn `SaveGameData`
  (params (SlotName :type String) (UserIndex :type Integer))
  (bind _returnvalue (`GameplayStatics.CreateSaveGameObject` "/Game/Blueprints/SaveGame/SaveGame_BP.SaveGame_BP_C"))
  (set `/Game/Blueprints/SaveGame/SaveGame_BP.SlotName` SlotName _returnvalue)
  (set `/Game/Blueprints/SaveGame/SaveGame_BP.UserIndex` UserIndex _returnvalue)
  (bind _output_get (set `self.CurSaveGameObject` _returnvalue))
  (bind _returnvalue_2 (`self.SaveDatasToString`))
  (set `/Game/Blueprints/SaveGame/SaveGame_BP.DataString` _returnvalue_2 _output_get)
  (bind _slotname (`/Game/Blueprints/SaveGame/SaveGame_BP.SlotName` _output_get))
  (bind _userindex (`/Game/Blueprints/SaveGame/SaveGame_BP.UserIndex` _output_get))
  (`GameplayStatics.SaveGameToSlot` _output_get _slotname _userindex)
  (set `self.CurSlotName` _slotname)
  (set `self.CurUserIndex` _userindex)
  (`KismetSystemLibrary.PrintString` "SaveGame Succe ================================================="))

(fn `SetData`
  (params (DataName :type String) (DataType :type "/Game/Blueprints/SaveGame/ESaveGameData Enum" :default "NewEnumerator0") (String :type String) (Integer :type Integer) (Float :type "Float (double-precision)") (Boolean :type Boolean) (Vector :type "Vector Structure"))
  (locals (LV_Data :type "/Game/Blueprints/SaveGame/SaveDataObject_BP Object Reference"))
  (bind _lv_data (`local.LV_Data`))
  (bind (_value _returnvalue) (`BlueprintMapLibrary.Map_Find` (`self.SaveDatas`) DataName))
  (if _returnvalue
    (`/Engine/EditorBlueprintResources/StandardMacros.IsValid` _value
      (:`Is Valid`
        (bind _output_get (set `local.LV_Data` _value))
        (if (`|EnumEquality` (`/Game/Blueprints/SaveGame/SaveDataObject_BP.DataType` _output_get) (`local.DataType`))
          (switch `/Game/Blueprints/SaveGame/ESaveGameData` (`local.DataType`)
            (:`NewEnumerator0`
              (set `/Game/Blueprints/SaveGame/SaveDataObject_BP.String` (`local.String`) (`local.LV_Data`)))
            (:`NewEnumerator1`
              (set `/Game/Blueprints/SaveGame/SaveDataObject_BP.Integer` (`local.Integer`) (`local.LV_Data`)))
            (:`NewEnumerator2`
              (set `/Game/Blueprints/SaveGame/SaveDataObject_BP.Float` (`local.Float`) (`local.LV_Data`)))
            (:`NewEnumerator3`
              (set `/Game/Blueprints/SaveGame/SaveDataObject_BP.Boolean` (`local.Boolean`) (`local.LV_Data`)))
            (:`NewEnumerator4`
              (set `/Game/Blueprints/SaveGame/SaveDataObject_BP.Vector` (`local.Vector`) (`local.LV_Data`))))
          (`/Game/Blueprints/SaveGame/SaveDataObject_BP.Event_ChangeValue` _lv_data _lv_data)
          (else
            (`KismetSystemLibrary.PrintString` "SaveDataType not equal")))))
    (else
      (`KismetSystemLibrary.PrintString` (`KismetStringLibrary.Concat_StrStr` DataName " not found")))))

(fn `StringToSaveDatas`
  (params (DataString :type String))
  (locals (LV_DataName :type String) (LV_DataType :type String) (LV_DataValue :type String))
  (bind _returnvalue (`KismetStringLibrary.ParseIntoArray` (`local.LV_DataValue`)))
  (`BlueprintMapLibrary.Map_Clear` (`self.SaveDatas`))
  (for _array_element (`KismetStringLibrary.ParseIntoArray` DataString ";")
    (bind _returnvalue_2 (`KismetStringLibrary.ParseIntoArray` _array_element ","))
    (set `local.LV_DataName` (`|GetArrayItem` _returnvalue_2))
    (set `local.LV_DataType` (`|GetArrayItem` _returnvalue_2 1))
    (set `local.LV_DataValue` (`|GetArrayItem` _returnvalue_2 2))
    (switch `string` (`local.LV_DataType`)
      (:`String`
        (`self.AddData` (`local.LV_DataName`) "NewEnumerator0" (`local.LV_DataValue`)))
      (:`Integer`
        (`self.AddData` (`local.LV_DataName`) "NewEnumerator1" "" (`KismetStringLibrary.Conv_StringToInt` (`local.LV_DataValue`))))
      (:`Float`
        (`self.AddData` (`local.LV_DataName`) "NewEnumerator2" "" 0 (`KismetStringLibrary.Conv_StringToDouble` (`local.LV_DataValue`))))
      (:`Bool`
        (switch `string` (`local.LV_DataValue`)
          (:`True`
            (`self.AddData` (`local.LV_DataName`) "NewEnumerator3" "" 0 0.0 true))
          (:`Flase`
            (`self.AddData` (`local.LV_DataName`) "NewEnumerator3"))))
      (:`Vector`
        (`self.AddData` (`local.LV_DataName`) "NewEnumerator4" "" 0 0.0 false (`KismetMathLibrary.MakeVector` (`KismetStringLibrary.Conv_StringToDouble` (`KismetStringLibrary.RightChop` (`|GetArrayItem` _returnvalue) 2)) (`KismetStringLibrary.Conv_StringToDouble` (`KismetStringLibrary.RightChop` (`|GetArrayItem` _returnvalue 1) 2)) (`KismetStringLibrary.Conv_StringToDouble` (`KismetStringLibrary.RightChop` (`|GetArrayItem` _returnvalue 2) 2)))))))
  (`KismetSystemLibrary.PrintString` (`KismetStringLibrary.Concat_StrStr` "There are " (`KismetStringLibrary.Conv_IntToString` (`BlueprintMapLibrary.Map_Length` (`self.SaveDatas`))) " pieces of Save data")))

(fn `UserConstructionScript`)