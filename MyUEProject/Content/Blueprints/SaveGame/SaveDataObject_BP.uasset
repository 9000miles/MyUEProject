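; SaveDataObject_BP is a save-game data object that holds a named value with a type tag.
; Its DataToString function switches on DataType to pick the matching String, Integer, Float, Boolean or Vector variable.
; It returns that value as a comma-separated record of name, type label and stringified value.
; The file contains only this serialization direction, with no parsing back from text.
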(fn `DataToString`
  (returns (Output :type String))
  (switch `/Game/Blueprints/SaveGame/ESaveGameData` (`self.DataType`)
    (:`NewEnumerator0`
      (return (`KismetStringLibrary.Concat_StrStr` (`self.DataName`) "," "String" "," (`self.String`))))
    (:`NewEnumerator1`
      (return (`KismetStringLibrary.Concat_StrStr` (`self.DataName`) "," "Integer" "," (`KismetStringLibrary.Conv_IntToString` (`self.Integer`)))))
    (:`NewEnumerator2`
      (return (`KismetStringLibrary.Concat_StrStr` (`self.DataName`) "," "Float" "," (`KismetStringLibrary.Conv_DoubleToString` (`self.Float`)))))
    (:`NewEnumerator3`
      (return (`KismetStringLibrary.Concat_StrStr` (`self.DataName`) "," "Boolean" "," (`KismetStringLibrary.Conv_BoolToString` (`self.Boolean`)))))
    (:`NewEnumerator4`
      (return (`KismetStringLibrary.Concat_StrStr` (`self.DataName`) "," "Vector" "," (`KismetStringLibrary.Conv_VectorToString` (`self.Vector`)))))))