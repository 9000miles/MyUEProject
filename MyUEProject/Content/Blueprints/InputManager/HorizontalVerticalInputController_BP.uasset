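; Input controller Blueprint that registers with InputManager_BP on BeginPlay, unregisters when destroyed, and turns received input into vertical and horizontal adjust events.
; Two AddInputAxisObjectBP helpers, sharing delay, speed and continuous-change settings, process forward and right axes separately.
; Each helper's value fires CallEventAdjustInput with the other axis zeroed.
; Key events forward only pressed state; both direction flags are false and the key comparisons are unconnected.
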(event `self.ReceiveBeginPlay`
  ;[1 1 1] 创建对象绑定输入
  (bind _returnvalue (`GameManager.GetManager` (subsystem `GameManager`) "/Game/Blueprints/Manager/InputManager_BP.InputManager_BP_C"))
  (bind _asinput_manager_bp (cast `/Game/Blueprints/Manager/InputManager_BP` _returnvalue))
  (`/Game/Blueprints/Manager/InputManager_BP.Func_AddTarget` _asinput_manager_bp self)
  (bind _returnvalue_2 (`AddComponent|NODE_AddInputAxisObject_BP-0` :`var_DelayTime` (`self.var_DelayTime`) :`var_Speed` (`self.var_Speed`) :`var_CanContinuousChange` (`self.var_CanContinuousChange`)))
  (bind _output_get (set `self.var_VerticalInput` _returnvalue_2))
  (add `/Game/Blueprints/InputManager/InputAxisObject_BP.Event_Value` _output_get (delegate `Event_VerticalValue`))
  (bind _returnvalue_3 (`AddComponent|NODE_AddInputAxisObject_BP-1` :`var_DelayTime` (`self.var_DelayTime`) :`var_Speed` (`self.var_Speed`) :`var_CanContinuousChange` (`self.var_CanContinuousChange`)))
  (bind _output_get_2 (set `self.var_HorizontalInput` _returnvalue_3))
  (add `/Game/Blueprints/InputManager/InputAxisObject_BP.Event_Value` _output_get_2 (delegate `Event_HorizontalValue`)))

(event `Event_VerticalValue`
  (params (Value :type Integer))
  ;[1 1 1] 创建对象绑定输入
  ;;[1 1 1] VerticalAxis
  (`self.Event_AdjustInput` Value))

(event `Event_HorizontalValue`
  (params (Value :type Integer))
  ;[1 1 1] 创建对象绑定输入
  ;;[1 1 1] HorizontalAxis
  (`self.Event_AdjustInput` 0 Value))

(event `/Game/Blueprints/InputManager/IBP_InputReceive.IBP_ReceiveAxis`
  (params (MoveForwardAxis :type "Float (single-precision)") (MoveRightAxis :type "Float (single-precision)") (LookUpAxis :type "Float (single-precision)") (LookRateAxis :type "Float (single-precision)"))
  ;[1 1 1] 输入轴
  (`|ExecutionSequence`
    (:`then_0`
      (`/Game/Blueprints/InputManager/InputAxisObject_BP.Func_InputAxis` (`self.var_VerticalInput`) MoveForwardAxis))
    (:`then_1`
      (`/Game/Blueprints/InputManager/InputAxisObject_BP.Func_InputAxis` (`self.var_HorizontalInput`) MoveRightAxis))))

(event `/Game/Blueprints/InputManager/IBP_InputReceive.IBP_ReceiveKey`
  (params (Key :type "/Game/Blueprints/InputManager/EInputKey Enum" :default "NewEnumerator0") (Pressed :type Boolean))
  ;[1 1 1] 方向键
  (`|ExecutionSequence`
    (:`then_0`
      (`/Game/Blueprints/InputManager/InputAxisObject_BP.Func_InputKey` (`self.var_VerticalInput`) false false Pressed))
    (:`then_1`
      (`/Game/Blueprints/InputManager/InputAxisObject_BP.Func_InputKey` (`self.var_HorizontalInput`) false false Pressed))))

(event `self.ReceiveDestroyed`
  ;[1 1 1] 解绑输入
  (bind _returnvalue (`GameManager.GetManager` (subsystem `GameManager`) "/Game/Blueprints/Manager/InputManager_BP.InputManager_BP_C"))
  (bind _asinput_manager_bp (cast `/Game/Blueprints/Manager/InputManager_BP` _returnvalue))
  (`/Game/Blueprints/Manager/InputManager_BP.Func_RemoveTarget` _asinput_manager_bp self))

(fn `UserConstructionScript`)