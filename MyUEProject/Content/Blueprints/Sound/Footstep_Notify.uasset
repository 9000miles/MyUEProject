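; Animation notify that plays a surface-dependent footstep sound when triggered by an animation.
; It traces straight down through the player character's location against static and physics objects, using complex collision.
; The hit physical material is cast to a custom type and its footstep sound is played as non-spatial 2D audio.
; It always samples player zero, not the mesh that fired the notify.
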(fn `Received_Notify`
  (params (MeshComp :type "SkeletalMeshComponent Object Reference") (Animation :type "AnimSequenceBase Object Reference"))
  (returns (ReturnValue :type Boolean))
  (bind _returnvalue (`Actor.K2_GetActorLocation` (`GameplayStatics.GetPlayerCharacter` 0)))
  (bind _outhit (`KismetSystemLibrary.LineTraceSingleForObjects` :`Start` (+ _returnvalue (0.0 0.0 200.0)) :`End` (- _returnvalue (0.0 0.0 2000.0)) :`ObjectTypes` (`|MakeArray` "ObjectTypeQuery1" "ObjectTypeQuery4" :!type "EObjectTypeQuery Enum") :`bTraceComplex` true :`DrawTime` 5000.0))
  (`|ExecutionSequence`
    (:`then_0`
      (bind _asground_physical_material (cast `` (`.PhysMat` (`GameplayStatics.BreakHitResult` _outhit))))
      (`GameplayStatics.PlaySound2D` (`/Game/Blueprints/Sound/Footstep_Notify.FootstepSound` _asground_physical_material) 1.0 1.0 0.0 null null)
      (return false))))