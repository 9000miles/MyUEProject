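; Sound manager that plays, pauses and stops sounds by ID, reading cue, fade times and restart flag from Sound_DT.
; Play spawns audio components, caching restartable ones as AudioObjects in an ID-keyed map for restarting, pausing and stopping with optional fades.
; A cleanup function destroys non-playing components and prunes the map.
; Numpad, Space and H keys exercise playback, pause and stop-all, while Tick prints component and map counts for debugging.
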(event `self.ReceiveTick`
  (params (DeltaSeconds :type "Float (single-precision)"))
  (bind _keys (`BlueprintMapLibrary.Map_Keys` (`self.var_AudioPlayerComDic`)))
  (`KismetSystemLibrary.PrintString` (`KismetStringLibrary.Concat_StrStr` (`KismetStringLibrary.Conv_IntToString` (`KismetArrayLibrary.Array_Length` (`self.K2_GetComponentsByClass` "/Script/Engine.AudioComponent"))) "------------" (`KismetStringLibrary.Conv_IntToString` (`KismetArrayLibrary.Array_Length` _keys)))))

(event `Key|NumPadZero`
  (params (Key :type "Key Structure"))
  (:`Pressed`
    (`self.Func_Play` "1000")))

(event `Key|NumPadOne`
  (params (Key :type "Key Structure"))
  (:`Pressed`
    (`self.Func_Play` "1001")))

(event `Key|NumPadTwo`
  (params (Key :type "Key Structure"))
  (:`Pressed`
    (`self.Func_Play` "1002")))

(event `Key|NumPadThree`
  (params (Key :type "Key Structure"))
  (:`Pressed`
    (`self.Func_Play` "1003")))

(event `Key|SpaceBar`
  (params (Key :type "Key Structure"))
  (:`Pressed`
    (`self.Func_Pause` "1001" true))
  (:`Released`
    (`self.Func_Pause` "1001")))

(event `Key|H`
  (params (Key :type "Key Structure"))
  (:`Pressed`
    (`self.Func_StopAll` true)))

(event `CustomEvent_0`
  (`KismetSystemLibrary.PrintString` "Hello"))

(fn `Func_Pause`
  (params (SoundID :type Name) (Pause :type Boolean))
  (locals (LV_SoundID :type Name))
  (bind (_value _returnvalue) (`BlueprintMapLibrary.Map_Find` (`self.var_AudioPlayerComDic`) (`local.LV_SoundID`)))
  (bind _var_audiocom (`/Game/BluePrints/SoundBP/AudioObject.var_AudioCom` _value))
  (set `local.LV_SoundID` SoundID)
  (if _returnvalue
    (`|GetDataTableRow` "/Game/BluePrints/SoundBP/Sound_DT.Sound_DT" (`local.LV_SoundID`)
      (:`then`
        (if Pause
          (`AudioComponent.SetPaused` _var_audiocom Pause)
          (bind _output_get (set `/Game/BluePrints/SoundBP/AudioObject.var_PauseTime` (- (`GameplayStatics.GetTimeSeconds`) (`/Game/BluePrints/SoundBP/AudioObject.var_StartTime` _value)) _value))
          (`KismetSystemLibrary.PrintString` (`KismetStringLibrary.Conv_DoubleToString` _output_get))
          (else
            (`AudioComponent.SetPaused` _var_audiocom Pause)))))))

(fn `Func_Play`
  (params (SoundID :type Name))
  (locals (LV_AudioCom :type "AudioComponent Object Reference") (LV_SoundID :type Name))
  (bind (_value _returnvalue) (`BlueprintMapLibrary.Map_Find` (`self.var_AudioPlayerComDic`) (`local.LV_SoundID`)))
  (set `local.LV_SoundID` SoundID)
  (bind _returnvalue_2 (`|GetDataTableRow` "/Game/BluePrints/SoundBP/Sound_DT.Sound_DT" (`local.LV_SoundID`))
    (:`then`
      (bind (_soundcue _isrestart _fadeintime) (break `/Game/BluePrints/SoundBP/Struct_Sound` _returnvalue_2))
      (if (and _returnvalue _isrestart)
        (`AudioComponent.FadeIn` (`/Game/BluePrints/SoundBP/AudioObject.var_AudioCom` _value) _fadeintime 1.0 0.0)
        (set `/Game/BluePrints/SoundBP/AudioObject.var_StartTime` (`GameplayStatics.GetTimeSeconds`) _value)
        (else
          (bind _returnvalue_3 (`AddComponent|NODE_AddAudioComponent-0`))
          (set `local.LV_AudioCom` _returnvalue_3)
          (bind _returnvalue_4 (`|GetDataTableRow` "/Game/BluePrints/SoundBP/Sound_DT.Sound_DT" (`local.LV_SoundID`))
            (:`then`
              (bind (_soundcue_2 _isrestart_2 _fadeintime_2 _fadeouttime) (break `/Game/BluePrints/SoundBP/Struct_Sound` _returnvalue_4))
              (`AudioComponent.SetSound` (`local.LV_AudioCom`) _soundcue_2)
              (`AudioComponent.FadeIn` (`local.LV_AudioCom`) _fadeintime_2 1.0 0.0)
              (if (not (not _isrestart_2))
                (bind _returnvalue_5 (`|GenericCreateObject` "/Game/BluePrints/SoundBP/AudioObject.AudioObject_C" self (`local.LV_AudioCom`) (`GameplayStatics.GetTimeSeconds`) _fadeintime_2 _fadeouttime))
                (`BlueprintMapLibrary.Map_Add` (`self.var_AudioPlayerComDic`) (`local.LV_SoundID`) _returnvalue_5))
              (add `AudioComponent.OnAudioFinished` (`local.LV_AudioCom`) (`|CreateDelegate` :!event `Func_RemoveAudioCom`)))))))))

(fn `Func_RemoveAudioCom`
  (locals (LV_AudioCom :type "AudioComponent Object Reference") (LV_SoundID :type Name) (LV_isCanRemove :type Boolean))
  (bind _lv_audiocom (`local.LV_AudioCom`))
  (bind _var_audioplayercomdic (`self.var_AudioPlayerComDic`))
  (bind (_value _returnvalue) (`BlueprintMapLibrary.Map_Find` (`self.var_AudioPlayerComDic`) (`local.LV_SoundID`)))
  (for _array_element (`self.K2_GetComponentsByClass` "/Script/Engine.AudioComponent")
    (set `local.LV_AudioCom` _array_element)
    (if (not (`AudioComponent.IsPlaying` _array_element))
      (set `local.LV_isCanRemove` true)
      (bind _keys (`BlueprintMapLibrary.Map_Keys` (`self.var_AudioPlayerComDic`)))
      (for _array_element_2 _keys
        (set `local.LV_SoundID` _array_element_2)
        (if _returnvalue
          (if (and (not (`/Game/BluePrints/SoundBP/AudioObject.var_IsPause` _value)) (== (`/Game/BluePrints/SoundBP/AudioObject.var_AudioCom` _value) (`local.LV_AudioCom`)))
            (set `local.LV_isCanRemove` true)
            (break)
            (else
              (set `local.LV_isCanRemove` false)))))
      (if (`local.LV_isCanRemove`)
        (`BlueprintMapLibrary.Map_Remove` _var_audioplayercomdic (`local.LV_SoundID`))
        (`ActorComponent.K2_DestroyComponent` (`local.LV_AudioCom`))
        (else
          (bind _values (`BlueprintMapLibrary.Map_Values` _var_audioplayercomdic))
          (for _array_element_3 _values
            (if (!= (`/Game/BluePrints/SoundBP/AudioObject.var_AudioCom` _array_element_3) (`local.LV_AudioCom`))
              (`/Engine/EditorBlueprintResources/StandardMacros.IsValid` _lv_audiocom
                (:`Is Valid`
                  (`ActorComponent.K2_DestroyComponent` _lv_audiocom))))))))))

(fn `Func_Stop`
  (params (SoundID :type Name) (ImmediatelyStop :type Boolean))
  (bind (_value _returnvalue) (`BlueprintMapLibrary.Map_Find` (`self.var_AudioPlayerComDic`) SoundID))
  (bind _var_audiocom (`/Game/BluePrints/SoundBP/AudioObject.var_AudioCom` _value))
  (if _returnvalue
    (bind _returnvalue_2 (`|GetDataTableRow` "/Game/BluePrints/SoundBP/Sound_DT.Sound_DT" SoundID)
      (:`then`
        (set `/Game/BluePrints/SoundBP/AudioObject.var_IsPause` false _value)
        (if (`local.ImmediatelyStop`)
          (`AudioComponent.Stop` _var_audiocom)
          (else
            (`AudioComponent.FadeOut` _var_audiocom (`.FadeOutTime_10_251B7D044AA5241963ACB8BE4711BDB7` (break `/Game/BluePrints/SoundBP/Struct_Sound` _returnvalue_2)) 0.0)))))))

(fn `Func_StopAll`
  (params (ImmediatelyStop :type Boolean))
  (bind _keys (`BlueprintMapLibrary.Map_Keys` (`self.var_AudioPlayerComDic`)))
  (for _array_element _keys
    (bind (_value _returnvalue) (`BlueprintMapLibrary.Map_Find` (`self.var_AudioPlayerComDic`) _array_element))
    (if _returnvalue
      (if (`local.ImmediatelyStop`)
        (bind _var_audiocom (`/Game/BluePrints/SoundBP/AudioObject.var_AudioCom` _value))
        (`AudioComponent.Stop` _var_audiocom)
        (else
          (`AudioComponent.FadeOut` _var_audiocom (`/Game/BluePrints/SoundBP/AudioObject.var_FadeOutTime` _value) 0.0)))))
  (`BlueprintMapLibrary.Map_Clear` (`self.var_AudioPlayerComDic`)))

(fn `UserConstructionScript`)