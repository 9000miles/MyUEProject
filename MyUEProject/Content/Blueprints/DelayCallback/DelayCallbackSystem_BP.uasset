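; Delay callback manager that fires timed, optionally looping callbacks carried by info objects.
; Callbacks register in a keyed map that rejects duplicate keys, or in an unkeyed array without setting a start time, and support removal by key, object or all at once.
; Tick polls both collections against game time, restarting repeats and removing finished entries; a non-positive loop count repeats indefinitely.
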(event `self.ReceiveTick`
  (params (DeltaSeconds :type "Float (single-precision)"))
  (`|ExecutionSequence`
    (:`then_0`
      (`self.Func_TickInfoDic`))
    (:`then_1`
      (`self.Func_TickInfoArray`))))

(event `CustomEvent_0`
  (`KismetSystemLibrary.PrintString` "0000000000000000000000000000000"))

(event `CustomEvent_1`
  (`KismetSystemLibrary.PrintString` "444444444444444444444444"))

(fn `Func_AddCallback`
  (params (Info :type "Object Object Reference") (InfoKey :type Name))
  (bind (_info _info_2) (`local.Info`))
  (if (not (== InfoKey "None"))
    (`/Engine/EditorBlueprintResources/StandardMacros.IsValid` Info
      (:`Is Valid`
        (if (not (`BlueprintMapLibrary.Map_Contains` (`.var_CallbackInfoDic` (`self.var_CallbackInfoDic`)) InfoKey))
          (set `/Game/Blueprints/DelayCallback/DelayCallbackSystem_BP.var_StartTime` (`GameplayStatics.GetTimeSeconds`) _info_2)
          (`BlueprintMapLibrary.Map_Add` (`.var_CallbackInfoDic` (`self.var_CallbackInfoDic`)) (`local.InfoKey`) _info_2)
          (else
            (`KismetSystemLibrary.PrintString` (`KismetStringLibrary.Concat_StrStr` (`KismetStringLibrary.Conv_NameToString` (`local.InfoKey`)) "is already exist"))))))
    (else
      (`KismetArrayLibrary.Array_Add` (`.var_CallbackInfoKeyNoneArray` (`self.var_CallbackInfoKeyNoneArray`)) (`.Info` (`local.Info`)))
      (`KismetSystemLibrary.PrintString` "Info key is None, Better not none in order to remove the CallbackInfo" true true (struct :`R` 1.0 :`B` 0.016184 :`A` 1.0)))))

(fn `Func_RemoveAll`
  (`BlueprintMapLibrary.Map_Clear` (`.var_CallbackInfoDic` (`self.var_CallbackInfoDic`)))
  (`KismetArrayLibrary.Array_Clear` (`.var_CallbackInfoKeyNoneArray` (`self.var_CallbackInfoKeyNoneArray`))))

(fn `Func_RemoveByInfo`
  (params (Info :type "Object Object Reference (by ref)"))
  (`|ExecutionSequence`
    (:`then_0`
      (bind _values (`BlueprintMapLibrary.Map_Values` (`.var_CallbackInfoDic` (`self.var_CallbackInfoDic`))))
      (if (`KismetArrayLibrary.Array_Contains` _values (`.Info` (`local.Info`)))
        (bind _keys (`BlueprintMapLibrary.Map_Keys` (`.var_CallbackInfoDic` (`self.var_CallbackInfoDic`))))
        (for _array_element _keys
          (bind (_value _returnvalue) (`BlueprintMapLibrary.Map_Find` (`.var_CallbackInfoDic` (`self.var_CallbackInfoDic`)) _array_element))
          (if (and (== _value (`.Info` (`local.Info`))) _returnvalue)
            (`BlueprintMapLibrary.Map_Remove` (`.var_CallbackInfoDic` (`self.var_CallbackInfoDic`)) _array_element)
            (break)))))
    (:`then_1`
      (if (`KismetArrayLibrary.Array_Contains` (`.var_CallbackInfoKeyNoneArray` (`self.var_CallbackInfoKeyNoneArray`)) (`.Info` (`local.Info`)))
        (`KismetArrayLibrary.Array_RemoveItem` (`.var_CallbackInfoKeyNoneArray` (`self.var_CallbackInfoKeyNoneArray`)) (`.Info` (`local.Info`)))))))

(fn `Func_RemoveByInfoKey`
  (params (InfoKey :type Name))
  (if (`BlueprintMapLibrary.Map_Contains` (`.var_CallbackInfoDic` (`self.var_CallbackInfoDic`)) InfoKey)
    (`BlueprintMapLibrary.Map_Remove` (`.var_CallbackInfoDic` (`self.var_CallbackInfoDic`)) InfoKey)))

(fn `Func_TickCallInfoEvent`
  (params (Info :type "Object Object Reference"))
  (returns (IsCanRemove :type Boolean))
  (bind (_info _info_2) (`local.Info`))
  (bind (_info_3 _info_4) (`local.Info`))
  (bind (_info_5 _info_6) (`local.Info`))
  (bind (_info_7 _info_8) (`local.Info`))
  (bind _output_get (set `/Game/Blueprints/DelayCallback/DelayCallbackSystem_BP.var_RemainingTime` (- (`GameplayStatics.GetTimeSeconds`) (+ (`/Game/Blueprints/DelayCallback/DelayCallbackSystem_BP.var_StartTime` _info_2) (`/Game/Blueprints/DelayCallback/DelayCallbackSystem_BP.var_DelayTime` _info_2))) Info))
  (`|ExecutionSequence`
    (:`then_0`
      (if (`/Game/Blueprints/DelayCallback/DelayCallbackSystem_BP.var_IsPrintTime` _info_4)
        (`KismetSystemLibrary.PrintString` (`KismetStringLibrary.Conv_DoubleToString` (`/Game/Blueprints/DelayCallback/DelayCallbackSystem_BP.var_RemainingTime` _info_4)))))
    (:`then_1`
      (if (>= _output_get 0.0)
        (`self.EventCallback` _info_6)
        (if (<= (`/Game/Blueprints/DelayCallback/DelayCallbackSystem_BP.var_LoopCount` _info_6) 0)
          (set `/Game/Blueprints/DelayCallback/DelayCallbackSystem_BP.var_StartTime` (`GameplayStatics.GetTimeSeconds`) (`.Info` (`local.Info`)))
          (return false)
          (else
            (bind _result (`/Engine/EditorBlueprintResources/StandardMacros.IncrementInt` (`/Game/Blueprints/DelayCallback/DelayCallbackSystem_BP.var_LoopNumber` _info_8))
              (:`  `
                (if (>= _result (`/Game/Blueprints/DelayCallback/DelayCallbackSystem_BP.var_LoopCount` _info_8))
                  (return true)
                  (else
                    (set `/Game/Blueprints/DelayCallback/DelayCallbackSystem_BP.var_StartTime` (`GameplayStatics.GetTimeSeconds`) (`.Info` (`local.Info`)))
                    (return false)))))))
        (else
          (return false))))))

(fn `Func_TickInfoArray`
  (for _array_element (`.var_CallbackInfoKeyNoneArray` (`self.var_CallbackInfoKeyNoneArray`))
    (`/Engine/EditorBlueprintResources/StandardMacros.IsValid` _array_element
      (:`Is Valid`
        (bind _iscanremove (`self.Func_TickCallInfoEvent` _array_element))
        (if _iscanremove
          (`KismetArrayLibrary.Array_RemoveItem` (`.var_CallbackInfoKeyNoneArray` (`self.var_CallbackInfoKeyNoneArray`)) _array_element))))))

(fn `Func_TickInfoDic`
  (bind _keys (`BlueprintMapLibrary.Map_Keys` (`.var_CallbackInfoDic` (`self.var_CallbackInfoDic`))))
  (for _array_element _keys
    (bind (_value _returnvalue) (`BlueprintMapLibrary.Map_Find` (`.var_CallbackInfoDic` (`self.var_CallbackInfoDic`)) _array_element))
    (if _returnvalue
      (`/Engine/EditorBlueprintResources/StandardMacros.IsValid` _value
        (:`Is Valid`
          (bind _iscanremove (`self.Func_TickCallInfoEvent` _value))
          (if _iscanremove
            (`BlueprintMapLibrary.Map_Remove` (`.var_CallbackInfoDic` (`self.var_CallbackInfoDic`)) _array_element)))))))

(fn `UserConstructionScript`)