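; CountdownGameOver_BP is a countdown actor that triggers a game-over transition when its delay expires.
; BeginPlay builds a callback info object bound to the timeout, and FuncStart registers it with the level's DelayCallback system.
; On timeout it binds itself as the player controller's locked message target, fades to black, waits, clears all widgets, then plays a configured sequence, clearing run data.
; Destruction releases the controller's message binding.
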(event `self.ReceiveBeginPlay`
  (bind _returnvalue (`|GenericCreateObject` "/Game/BluePrints/PublicBP/DelayCallback/CallbackInfo_BP.CallbackInfo_BP_C" self (`self.var_DelayTime`)))
  (add `/Game/BluePrints/PublicBP/DelayCallback/CallbackInfo_BP.EventCallback` _returnvalue (delegate `Event_TimeOut`))
  (set `self.var_CallbackInfo` _returnvalue))

(event `Event_TimeOut`
  (message `/Game/BluePrints/InterfaceBP/IBP_InputKey.IBP_BindReceiveTarge` (`GameplayStatics.GetPlayerController` 0) self true)
  (bind _returnvalue (`|CreateWidget` "/Game/UIWidget/GradientBlackScreen_Widget.GradientBlackScreen_Widget_C"))
  (`/Game/UIWidget/GradientBlackScreen_Widget.Func_Show` _returnvalue (/ 1.0 (`self.var_FadeTime`)))
  (`KismetSystemLibrary.Delay` (+ (`self.var_FadeTime`) (`self.var_StandingTime`)))
  (`Widget.RemoveFromParent` _returnvalue)
  (`WidgetLayoutLibrary.RemoveAllWidgets`)
  (bind _outactors (`GameplayStatics.GetAllActorsOfClass` "/Game/BluePrints/ManaMovieBP/SeqManaManagerBP.SeqManaManagerBP_C"))
  (`/Game/BluePrints/ManaMovieBP/SeqManaManagerBP.Func_SetWidgetZoder` (`|GetArrayItem` _outactors) 4)
  (`/Game/BluePrints/BP_Sequence/FunctionLibrary_Sequence.Func_StartPlaySequence` (`self.var_SequenceIndex`)))

(event `self.ReceiveDestroyed`
  (message `/Game/BluePrints/InterfaceBP/IBP_InputKey.IBP_RemoveReceiveTarget` (`GameplayStatics.GetPlayerController` 0) self))

(fn `Func_Start`
  (bind _outactors (`GameplayStatics.GetAllActorsOfClass` "/Game/BluePrints/PublicBP/DelayCallback/DelayCallbackSystem_BP.DelayCallbackSystem_BP_C"))
  (`/Game/BluePrints/PublicBP/DelayCallback/DelayCallbackSystem_BP.Func_AddCallback` (`|GetArrayItem` _outactors) (`self.var_CallbackInfo`)))

(fn `UserConstructionScript`)