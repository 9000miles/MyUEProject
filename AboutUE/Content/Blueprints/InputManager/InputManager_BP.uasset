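; Input manager that relays Jump and Crouch keys and movement and look-up axes to registered targets through interface messages.
; Register and unregister events maintain a list of InputTarget_BP wrappers holding each target and an authority value, which broadcasts ignore.
; Each axis event updates its cached value, then sends all four cached axes to every target, even when unchanged.
; Turn and TurnRate are unhandled.
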(event `InputAction|Jump`
  (params (Key :type "Key Structure"))
  (:`Pressed`
    (`self.Func_BroadcastInputKey` "NewEnumerator4" true))
  (:`Released`
    (`self.Func_BroadcastInputKey` "NewEnumerator4")))

(event `InputAction|Crouch`
  (params (Key :type "Key Structure"))
  (:`Pressed`
    (`self.Func_BroadcastInputKey` "NewEnumerator5" true))
  (:`Released`
    (`self.Func_BroadcastInputKey` "NewEnumerator5")))

(event `InputAxis|MoveForward`
  (params (AxisValue :type "Float (single-precision)"))
  (`self.Func_BroadcastInputAxis` "MoveForward" AxisValue))

(event `InputAxis|MoveRight`
  (params (AxisValue :type "Float (single-precision)"))
  (`self.Func_BroadcastInputAxis` "MoveRight" AxisValue))

(event `InputAxis|LookUp`
  (params (AxisValue :type "Float (single-precision)"))
  (`self.Func_BroadcastInputAxis` "LookUp" AxisValue))

(event `InputAxis|LookUpRate`
  (params (AxisValue :type "Float (single-precision)"))
  (`self.Func_BroadcastInputAxis` "LookUpRate" AxisValue))

(event `InputAxis|Turn`
  (params (AxisValue :type "Float (single-precision)")))

(event `InputAxis|TurnRate`
  (params (AxisValue :type "Float (single-precision)")))

(event `/Game/Blueprints/InputManager/InputInterface_IBP.IBP_RegisterInput`
  (params (Target :type "Object Object Reference") (Authority :type "/Game/Blueprints/InputManager/EInputAuthority Enum" :default "NewEnumerator0"))
  (bind _returnvalue (`|GenericCreateObject` "/Game/Blueprints/InputManager/InputTarget_BP.InputTarget_BP_C" self Target Authority))
  (`KismetArrayLibrary.Array_AddUnique` (`self.InputTargets`) _returnvalue))

(event `/Game/Blueprints/InputManager/InputInterface_IBP.IBP_UnregisterInput`
  (params (Target :type "Object Object Reference"))
  (bind _inputtargets (`self.InputTargets`))
  (for _array_element _inputtargets
    (if (== (`/Game/Blueprints/InputManager/InputTarget_BP.Target` _array_element) Target)
      (`KismetArrayLibrary.Array_RemoveItem` _inputtargets _array_element))))

(event `IBP_Init_1`
  (params (Key :type Name))
  (switch `string` (`KismetStringLibrary.RightPad` (`KismetStringLibrary.Conv_NameToString` Key) 1)))

(fn `Func_BroadcastInputAxis`
  (params (AxisName :type Name) (Axis :type "Float (double-precision)"))
  (switch `name` AxisName
    (:`MoveForward`
      (if (!= Axis (`self.MoveForwardAxis`))
        (set `self.MoveForwardAxis` Axis)))
    (:`MoveRight`
      (if (!= Axis (`self.MoveRightAxis`))
        (set `self.MoveRightAxis` Axis)))
    (:`LookUp`
      (if (!= Axis (`self.LookUpAxis`))
        (set `self.LookUpAxis` Axis)))
    (:`LookUpRate`
      (if (!= Axis (`self.LookUpRateAxis`))
        (set `self.LookUpRateAxis` Axis))))
  (for _array_element (`self.InputTargets`)
    (message `/Game/Blueprints/InputManager/InputInterface_IBP.IBP_ReceiveAxis` (`/Game/Blueprints/InputManager/InputTarget_BP.Target` _array_element) (`self.MoveForwardAxis`) (`self.MoveRightAxis`) (`self.LookUpAxis`) (`self.LookUpRateAxis`))))

(fn `Func_BroadcastInputKey`
  (params (Key :type "/Game/Blueprints/InputManager/EInputKey Enum" :default "NewEnumerator0") (Pressed :type Boolean))
  (for _array_element (`self.InputTargets`)
    (message `/Game/Blueprints/InputManager/InputInterface_IBP.IBP_ReceiveKey` (`/Game/Blueprints/InputManager/InputTarget_BP.Target` _array_element) Key Pressed)))

(fn `UserConstructionScript`)