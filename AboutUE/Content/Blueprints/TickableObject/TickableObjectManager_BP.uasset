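; TickableObjectManager_BP is a central tick dispatcher that drives per-frame updates for registered objects.
; Objects are added uniquely to an array, removed individually or cleared all at once through its functions.
; Each Tick, it loops over the array and calls TickMessage with DeltaSeconds on every valid entry, skipping invalid ones without removing them.
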(event `self.ReceiveTick`
  (params (DeltaSeconds :type "Float (single-precision)"))
  (for _array_element (`self.TickObjectArrary`)
    (`/Engine/EditorBlueprintResources/StandardMacros.IsValid` _array_element
      (:`Is Valid`
        (message `/Game/Blueprints/TickableObject/Tickable_IBP.Tick` _array_element DeltaSeconds)))))

(fn `AddTickObject`
  (params (Item :type "Object Object Reference (by ref)"))
  (`KismetArrayLibrary.Array_AddUnique` (`self.TickObjectArrary`) Item))

(fn `ClearTickArrary`
  (`KismetArrayLibrary.Array_Clear` (`self.TickObjectArrary`)))

(fn `RemoveTickObject`
  (params (Item :type "Object Object Reference (by ref)"))
  (`KismetArrayLibrary.Array_RemoveItem` (`self.TickObjectArrary`) Item))

(fn `UserConstructionScript`)