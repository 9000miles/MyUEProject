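; Input helper object that turns a positive/negative key pair or an analog axis into discrete +1, -1 and 0 value events.
; A key press or threshold crossing fires once, then a delay timer starts looping timers that repeat the step if continuous change is enabled.
; The axis re-arms within a middle dead zone, with extra side tracking intended for direct flips between extremes.
; Delay, repeat interval and continuous change are configurable.
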(fn `Func_InputAxis`
  (params (Axis :type "Float (double-precision)"))
  (bind _var_isaxismiddle (`self.var_IsAxisMiddle`))
  (bind _returnvalue (<= Axis (`self.var_AxisMin`)))
  (bind _returnvalue_2 (not (`self.var_HasCallEvent`)))
  (`|ExecutionSequence`
    (:`then_0`
      (if (and _returnvalue _var_isaxismiddle)
        (set `self.var_IsAxisMiddle` false)
        (set `self.var_IsArrivedPositive` false)
        (set `self.var_IsArrivedNegative` true)
        (if _returnvalue_2
          (`self.Event_Value` -1)
          (set `self.var_HasCallEvent` true :!label _label)
          (set `self.var_IsKeyEvent` false)
          (`self.Func_StartDelay`))))
    (:`then_1`
      (if (and _var_isaxismiddle (>= Axis (`self.var_AxisMax`)))
        (set `self.var_IsAxisMiddle` false)
        (set `self.var_IsArrivedPositive` true)
        (set `self.var_IsArrivedNegative` false)
        (if _returnvalue_2
          (`self.Event_Value` 1)
          (goto _label))))
    (:`then_2`
      (if (<= (`KismetMathLibrary.Abs` Axis) (`self.var_AxisMiddleValue`))
        (set `self.var_IsAxisMiddle` true)
        (set `self.var_IsArrivedPositive` false)
        (set `self.var_IsArrivedNegative` false)
        (set `self.var_HasCallEvent` false)
        (`KismetSystemLibrary.K2_ClearTimer` null "Func_PositiveAxisChange")
        (`KismetSystemLibrary.K2_ClearTimer` null "Func_NegativeAxisChange")
        (`self.Event_Value` 0)))
    (:`then_3`
      ;[1 1 1] 处理直接从1跳到-1的情况
      (if _returnvalue
        (set `self.var_IsCurPositiveSide` true)
        (else
          (set `self.var_IsCurPositiveSide` false)))
      (if (!= (`self.var_IsCurPositiveSide`) (`self.var_LastSide`))
        (set `self.var_LastSide` (`self.var_IsCurPositiveSide`))
        (set `self.var_IsAxisMiddle` true))
      (`self.Event_Value` 0))))

(fn `Func_InputKey`
  (params (IsPositiveKeyDown :type Boolean) (IsNegativeKeyDown :type Boolean) (IsPressed :type Boolean))
  (set `self.var_IsPositiveKeyPressed` false)
  (set `self.var_IsNegativeKeyPressed` false)
  (`KismetSystemLibrary.K2_ClearTimer` null "Func_PositiveKeyChange")
  (`KismetSystemLibrary.K2_ClearTimer` null "Func_NegativeKeyChange")
  (`|ExecutionSequence`
    (:`then_0`
      (if (and IsPositiveKeyDown IsPressed)
        (set `self.var_IsPositiveKeyPressed` true)
        (set `self.var_IsNegativeKeyPressed` false)
        (`self.Event_Value` 1)
        (set `self.var_IsKeyEvent` true :!label _label)
        (`self.Func_StartDelay`)))
    (:`then_1`
      (if (and IsNegativeKeyDown IsPressed)
        (set `self.var_IsPositiveKeyPressed` false)
        (set `self.var_IsNegativeKeyPressed` true)
        (`self.Event_Value` -1)
        (goto _label)))))

(fn `Func_NegativeAxisChange`
  (if (`self.var_IsArrivedNegative`)
    (`self.Event_Value` -1)))

(fn `Func_NegativeKeyChange`
  (if (`self.var_IsNegativeKeyPressed`)
    (`self.Event_Value` -1)))

(fn `Func_PositiveAxisChange`
  (if (`self.var_IsArrivedPositive`)
    (`self.Event_Value` 1)))

(fn `Func_PositiveKeyChange`
  (if (`self.var_IsPositiveKeyPressed`)
    (`self.Event_Value` 1)))

(fn `Func_SetVariable`
  (params (var_DelayTime :type "Float (double-precision)") (var_Speed :type "Float (double-precision)") (var_CanContinuousChange :type Boolean))
  (set `self.var_DelayTime` var_DelayTime)
  (set `self.var_Speed` var_Speed)
  (set `self.var_CanContinuousChange` var_CanContinuousChange))

(fn `Func_StartChange`
  (if (`self.var_CanContinuousChange`)
    (if (`self.var_IsKeyEvent`)
      (`KismetSystemLibrary.K2_SetTimer` null "Func_PositiveKeyChange" (`self.var_Speed`) true)
      (`KismetSystemLibrary.K2_SetTimer` null "Func_NegativeKeyChange" (`self.var_Speed`) true)
      (else
        (`KismetSystemLibrary.K2_SetTimer` null "Func_PositiveAxisChange" (`self.var_Speed`) true)
        (`KismetSystemLibrary.K2_SetTimer` null "Func_NegativeAxisChange" (`self.var_Speed`) true)))))

(fn `Func_StartDelay`
  (`KismetSystemLibrary.K2_SetTimer` null "Func_StartChange" (`self.var_DelayTime`)))