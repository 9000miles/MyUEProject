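; HorizontalVerticalInputController_BP is an input controller actor meant to turn axis and key input into vertical and horizontal adjust events.
; Its two value handlers call CallEventAdjustInput with one axis filled and the other zero.
; Construction and binding of two InputAxisObject_BP helpers, with delay, speed and continuous-change settings, sit unwired, as do their key and axis feeds.
; BeginPlay, Destroyed and both input interface events therefore do nothing.
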(event `self.ReceiveBeginPlay`
  ;[1 1 1] 创建对象绑定输入
)

(event `Event_VerticalValue` :!signature `self.Event_Value`
  (params (Value :type Integer))
  ;[1 1 1] 创建对象绑定输入
  ;;[1 1 1] VerticalAxis
  (`self.Event_AdjustInput` Value))

(event `Event_HorizontalValue` :!signature `self.Event_Value`
  (params (Value :type Integer))
  ;[1 1 1] 创建对象绑定输入
  ;;[1 1 1] HorizontalAxis
  (`self.Event_AdjustInput` 0 Value))

(event `IBP_GetInputAxis_1`
  (params (ForwardAxis :type "Float (double-precision)") (RightAxis :type "Float (double-precision)"))
  ;[1 1 1] 输入轴
  (`|ExecutionSequence`))

(event `IBP_GetSignleInputKey_1`
  (params (Key :type Byte) (Pressed :type Boolean))
  ;[1 1 1] 方向键
  (`|ExecutionSequence`))

(event `self.ReceiveDestroyed`
  ;[1 1 1] 解绑输入
)

(fn `UserConstructionScript`)