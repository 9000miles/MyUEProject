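; DelayCallbackSystem_BP is a timer system that fires callbacks on registered info objects once their delay has elapsed.
; Adding an info stamps its start time and stores it without duplicates, and further functions remove one or clear all.
; Tick polls entries against game time, optionally prints the offset from the due time, then calls and removes due ones during the loop.
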(event `self.ReceiveTick`
  (params (DeltaSeconds :type "Float (single-precision)"))
  (for _array_element _
    (`/Engine/EditorBlueprintResources/StandardMacros.IsValid` _array_element
      (:`Is Valid`
        (bind _output_get (set `/Game/Blueprints/DelayCallback/DelayCallbackSystem_BP.var_RemainingTime` (- (`GameplayStatics.GetTimeSeconds`) (+ (`/Game/Blueprints/DelayCallback/DelayCallbackSystem_BP.var_StartTime` _array_element) (`/Game/Blueprints/DelayCallback/DelayCallbackSystem_BP.var_DelayTime` _array_element))) _array_element))
        (`|ExecutionSequence`
          (:`then_0`
            (if (`/Game/Blueprints/DelayCallback/DelayCallbackSystem_BP.var_IsPrintTime` _array_element)
              (`KismetSystemLibrary.PrintString` (`KismetStringLibrary.Conv_DoubleToString` _output_get))))
          (:`then_1`
            (if (>= _output_get 0.0)
              (`self.EventCallback` _array_element)
              (`KismetArrayLibrary.Array_RemoveItem` (`.var_CallbackInfos` (`self.var_CallbackInfos`)) _array_element))))))))

(fn `Func_AddCallback`
  (params (Info :type "Object Object Reference (by ref)"))
  (if (not (`KismetArrayLibrary.Array_Contains` :`ItemToFind` Info))
    (set `/Game/Blueprints/DelayCallback/DelayCallbackSystem_BP.var_StartTime` (`GameplayStatics.GetTimeSeconds`) Info)
    (`KismetArrayLibrary.Array_Add` :`NewItem` Info)))

(fn `Func_RemoveAll`
  (`KismetArrayLibrary.Array_Clear` (`.var_CallbackInfos` (`self.var_CallbackInfos`))))

(fn `Func_RemoveCallback`
  (params (Info :type "Object Object Reference (by ref)"))
  (bind (_var_callbackinfos _var_callbackinfos_2) (`self.var_CallbackInfos`))
  (if (`KismetArrayLibrary.Array_Contains` _var_callbackinfos_2 Info)
    (`KismetArrayLibrary.Array_RemoveItem` _var_callbackinfos_2 Info)))

(fn `UserConstructionScript`)