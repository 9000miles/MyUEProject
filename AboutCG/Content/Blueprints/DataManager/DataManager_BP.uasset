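; DataManager_BP is an actor that constructs a DataBase object on BeginPlay and carries debug-style key bindings for exercising the tickable manager.
; Numpad 1 and 7 each construct a BBB object and register it for ticking, while 2 and 8 remove the respective object.
; Numpad 5 clears the manager's tick array.
; An unconnected lookup of TickableObjectManager_BP through the actor manager never runs.
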(event `self.ReceiveBeginPlay`
  (`|GenericCreateObject` "/Game/Blueprints/DataManager/DataBase.DataBase_C" self))

(event `Key|NumPadOne`
  (params (Key :type "Key Structure"))
  (:`Pressed`
    (bind _returnvalue (`|GenericCreateObject` "/Game/Blueprints/Test/BBB.BBB_C" self))
    (bind _manager_bp (`/Game/Blueprints/FunctionLibrary/Manager_FL.FL_GetTickableManager`))
    (`/Game/Blueprints/TickableObject/TickableObjectManager_BP.AddTickObject` _manager_bp _returnvalue)))

(event `Key|NumPadTwo`
  (params (Key :type "Key Structure"))
  (:`Pressed`
    (bind _manager_bp (`/Game/Blueprints/FunctionLibrary/Manager_FL.FL_GetTickableManager`))
    (`/Game/Blueprints/TickableObject/TickableObjectManager_BP.RemoveTickObject` _manager_bp (stale `Key|NumPadOne` _returnvalue))))

(event `Key|NumPadSeven`
  (params (Key :type "Key Structure"))
  (:`Pressed`
    (bind _returnvalue (`|GenericCreateObject` "/Game/Blueprints/Test/BBB.BBB_C" self))
    (bind _manager_bp (`/Game/Blueprints/FunctionLibrary/Manager_FL.FL_GetTickableManager`))
    (`/Game/Blueprints/TickableObject/TickableObjectManager_BP.AddTickObject` _manager_bp _returnvalue)))

(event `Key|NumPadEight`
  (params (Key :type "Key Structure"))
  (:`Pressed`
    (bind _manager_bp (`/Game/Blueprints/FunctionLibrary/Manager_FL.FL_GetTickableManager`))
    (`/Game/Blueprints/TickableObject/TickableObjectManager_BP.RemoveTickObject` _manager_bp (stale `Key|NumPadSeven` _returnvalue))))

(event `Key|NumPadOne`
  (params (Key :type "Key Structure")))

(event `Key|NumPadFive`
  (params (Key :type "Key Structure"))
  (:`Pressed`
    (bind _manager_bp (`/Game/Blueprints/FunctionLibrary/Manager_FL.FL_GetTickableManager`))
    (`/Game/Blueprints/TickableObject/TickableObjectManager_BP.ClearTickArrary` _manager_bp)))

(fn `UserConstructionScript`)