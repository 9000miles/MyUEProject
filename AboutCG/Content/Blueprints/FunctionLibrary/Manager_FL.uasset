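; Blueprint function library that gives global access to the game's manager objects.
; FLGetManager reads the central ManagerActor stored on GameInstance_BP, printing an error if the cast fails.
; The other getters look up the data, tickable-object and input managers on it by name and cast each to its type.
; Input managers are resolved per index by appending the index to the lookup name.
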(fn `FL_GetDataManager`
  (returns (`Manager BP` :type "/Game/Blueprints/DataManager/DataManager_BP Object Reference"))
  (bind _manager_bp (`self.FL_GetManager` null))
  (bind _value (`/Game/Blueprints/Manager/Manager_BP.GetManager` _manager_bp "DataManager"))
  (bind _asdata_manager_bp (cast `/Game/Blueprints/DataManager/DataManager_BP` _value))
  (return _asdata_manager_bp))

(fn `FL_GetInputManager`
  (params (Index :type String))
  (returns (`Manager BP` :type "/Game/Blueprints/InputManager/InputManager_BP Object Reference"))
  (bind _manager_bp (`self.FL_GetManager` null))
  (bind _value (`/Game/Blueprints/Manager/Manager_BP.GetManager` _manager_bp (`KismetStringLibrary.Conv_StringToName` (`KismetStringLibrary.Concat_StrStr` "InputManager" "_" Index))))
  (bind _asinput_manager_bp (cast `/Game/Blueprints/InputManager/InputManager_BP` _value))
  (return _asinput_manager_bp))

(fn `FL_GetManager`
  (returns (`Manager BP` :type "/Game/Blueprints/Manager/Manager_BP Object Reference"))
  (bind _asgame_instance_bp (cast `/Game/Blueprints/GameSetting/GameInstance_BP` (`GameplayStatics.GetGameInstance` null))
    (:`then`
      (return (`/Game/Blueprints/GameSetting/GameInstance_BP.ManagerActor` _asgame_instance_bp)))
    (:`CastFailed`
      (`KismetSystemLibrary.PrintString` null "GameInstance cast failed"))))

(fn `FL_GetTickableManager`
  (returns (`Manager BP` :type "/Game/Blueprints/TickableObject/TickableObjectManager_BP Object Reference"))
  (bind _manager_bp (`self.FL_GetManager` null))
  (bind _value (`/Game/Blueprints/Manager/Manager_BP.GetManager` _manager_bp "TickableManager"))
  (bind _astickable_object_manager_bp (cast `/Game/Blueprints/TickableObject/TickableObjectManager_BP` _value))
  (return _astickable_object_manager_bp))