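; Manager_BP is a singleton-style hub actor that creates and tracks the game's manager actors by key.
; On BeginPlay it destroys itself if another copy exists, otherwise it spawns the input, data and tickable-object managers.
; Each spawned manager is cast to ManagerBase_BP, initialized with its key and stored in the ManagerDic map.
; Functions add, look up, remove or clear managers, printing messages for duplicate or missing keys.
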(event `self.ReceiveBeginPlay`
  (bind _outactors (`GameplayStatics.GetAllActorsOfClass` "Manager_BP_C"))
  (if (> (`KismetArrayLibrary.Array_Length` _outactors) 1)
    (`self.K2_DestroyActor`)
    (else
      (`self.InitManagers`))))

(fn `AddManager`
  (params (Key :type Name) (ValueClass :type "Actor Class Reference"))
  (returns (ReturnValue :type "Actor Object Reference"))
  (if (`.ReturnValue` (`BlueprintMapLibrary.Map_Find` (`self.ManagerDic`) Key))
    (`KismetSystemLibrary.PrintString` (`KismetStringLibrary.Concat_StrStr` (`KismetStringLibrary.Conv_NameToString` (`local.Key`)) " already existed"))
    (return null)
    (else
      (bind _returnvalue (`|SpawnActorFromClass` (`local.ValueClass`) (`KismetMathLibrary.MakeTransform` (0.0 0.0 0.0)) "AlwaysSpawn" "OverrideRootScale" null null))
      (bind _asmanager_base_bp (cast `/Game/Blueprints/Manager/ManagerBase_BP` _returnvalue))
      (`/Game/Blueprints/Manager/ManagerBase_BP.Func_Init` _asmanager_base_bp (`local.Key`))
      (`BlueprintMapLibrary.Map_Add` (`self.ManagerDic`) (`local.Key`) _asmanager_base_bp)
      (return _returnvalue))))

(fn `ClearAllManager`
  (bind _values (`BlueprintMapLibrary.Map_Values` (`self.ManagerDic`)))
  (for _array_element _values
    (`self.K2_DestroyActor` _array_element))
  (`BlueprintMapLibrary.Map_Clear` (`self.ManagerDic`)))

(fn `GetManager`
  (params (Key :type Name))
  (returns (Value :type "Actor Object Reference"))
  (bind (_value _returnvalue) (`BlueprintMapLibrary.Map_Find` (`self.ManagerDic`) Key))
  (if _returnvalue
    (`/Engine/EditorBlueprintResources/StandardMacros.IsValid` _value
      (:`Is Valid`
        (return _value))
      (:`Is Not Valid`
        (return null)))
    (else
      (`KismetSystemLibrary.PrintString` (`KismetStringLibrary.Concat_StrStr` (`KismetStringLibrary.Conv_NameToString` Key) " inexistence ")))))

(fn `InitManagers`
  (`self.AddManager` "InputManager_0" "/Game/Blueprints/InputManager/InputManager_BP.InputManager_BP_C")
  (`self.AddManager` "DataManager" "/Game/Blueprints/DataManager/DataManager_BP.DataManager_BP_C")
  (`self.AddManager` "TickableManager" "/Game/Blueprints/TickableObject/TickableObjectManager_BP.TickableObjectManager_BP_C"))

(fn `RemoveManager`
  (params (Key :type Name))
  (bind (_value _returnvalue) (`BlueprintMapLibrary.Map_Find` (`self.ManagerDic`) Key))
  (if _returnvalue
    (`BlueprintMapLibrary.Map_Remove` (`self.ManagerDic`) (`local.Key`))
    (`self.K2_DestroyActor` _value)
    (else
      (`KismetSystemLibrary.PrintString` (`KismetStringLibrary.Concat_StrStr` (`KismetStringLibrary.Conv_NameToString` (`local.Key`)) " inexistence")))))

(fn `UserConstructionScript`)